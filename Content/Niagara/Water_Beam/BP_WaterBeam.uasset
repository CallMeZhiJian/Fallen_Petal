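; BP_WaterBeam is a water beam projectile actor that damages enemies on impact.
; On hit, it applies fixed damage to actors tagged Enemy, spawns the P_Explosion emitter at its location and destroys itself, whatever it struck.
; BeginPlay also destroys it after a short delay, limiting its lifetime if it hits nothing.
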(event Collision|EventActorBeginOverlap
  (params (OtherActor :type Actor%20Object%20Reference)))

(event EventTick
  (params (DeltaSeconds :type Float%20%28single-precision%29)))

(event Collision|EventHit
  (params (MyComp :type Primitive%20Component%20Object%20Reference) (Other :type Actor%20Object%20Reference) (OtherComp :type Primitive%20Component%20Object%20Reference) (bSelfMoved :type Boolean) (HitLocation :type Vector :default "0, 0, 0") (HitNormal :type Vector :default "0, 0, 0") (NormalImpulse :type Vector :default "0, 0, 0") (Hit :type Hit%20Result%20Structure%20%28by%20ref%29))
  (if (Actor|ActorHasTag Other "Enemy")
    (Game|Damage|ApplyDamage Other 1e+01 0 0))
  (Effects|SpawnEmitteratLocation "/Game/StarterContent/Particles/P_Explosion.P_Explosion" (Transformation|GetActorLocation))
  (Utilities|IsValid self
    (:Is%20Valid
      (Actor|DestroyActor))))

(event EventBeginPlay
  (Utilities|FlowControl|Delay 2.0)
  (Utilities|IsValid self
    (:Is%20Valid
      (Actor|DestroyActor))))

(fn ConstructionScript)