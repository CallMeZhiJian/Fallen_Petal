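; BP_BossZone is a trigger zone that shows a boss health bar while the player is inside it.
; On overlap begin, it confirms the actor is the player's BP_KW_Testing character, has it spawn the bar for BossRef, and also applies a small hit of damage to the player.
; On overlap end, the same player check tells the character to remove the bar.
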(event EventBeginPlay)

(event Collision|EventActorBeginOverlap
  (params (OtherActor :type Actor%20Object%20Reference))
  (bind _asbp_kw_testing (Utilities|Casting|CastToBP_KW_Testing (Game|GetPlayerCharacter 0)))
  (if (== _asbp_kw_testing OtherActor)
    (Default|SpawnBossHealthBar _asbp_kw_testing (Variables|Default|GetBossRef))
    (Game|Damage|ApplyDamage _asbp_kw_testing 1e+01 0 0)))

(event Collision|EventActorEndOverlap
  (params (OtherActor :type Actor%20Object%20Reference))
  (bind _asbp_kw_testing (Utilities|Casting|CastToBP_KW_Testing (Game|GetPlayerCharacter 0)))
  (if (== _asbp_kw_testing OtherActor)
    (Default|RemoveBossHealthBar _asbp_kw_testing)))

(fn ConstructionScript)