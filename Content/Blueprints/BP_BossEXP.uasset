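; BP_BossEXP is an experimental boss Blueprint that exercises a HealthSystem component and sets a placeholder boss name on BeginPlay.
; The component's health-change and depletion events only print debug messages.
; LoseHealth subtracts from the component's Health directly, but the looping timer meant to call it is disconnected, so the drain never runs.
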(event OnHealthChange(HealthSystem)
  (params (NewHealth :type Float%20%28double-precision%29))
  (Development|PrintString (Utilities|String|Append "NewHealth:" (Utilities|String|ToString(Float) NewHealth))))

(event OnHealthDepleted(HealthSystem)
  (Development|PrintString "Character Died"))

(event Collision|EventActorBeginOverlap
  (params (OtherActor :type Actor%20Object%20Reference)))

(event EventTick
  (params (DeltaSeconds :type Float%20%28single-precision%29)))

(event EventBeginPlay
  (Variables|Default|SetBossName "Testing 123"))

(fn ConstructionScript)

(fn LoseHealth
  (bind _healthsystem (Variables|Default|GetHealthSystem))
  (Variables|/Game/Widget/HealthSystem.HealthSystem_C|SetHealth _healthsystem (- (Variables|/Game/Widget/HealthSystem.HealthSystem_C|GetHealth _healthsystem) 1.0)))