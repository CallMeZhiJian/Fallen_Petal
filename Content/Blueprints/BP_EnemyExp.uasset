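; BP_EnemyExp is an enemy Blueprint with a HealthSystem and a boss name, apparently a test setup for a boss health bar.
; BeginPlay only sets BossName to a placeholder string.
; LoseHealth decrements HealthSystem health by one, but the looping timer meant to call it is disconnected.
; The logic pushing health into the WB_BossHealthBar widget is also unwired, so neither runs.
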(event EventTick
  (params (DeltaSeconds :type Float%20%28single-precision%29)))

(event EventBeginPlay
  (Variables|Default|SetBossName "Testing 123"))

(fn ConstructionScript)

(fn LoseHealth
  (bind _healthsystem (Variables|Default|GetHealthSystem))
  (Variables|/Game/Widget/HealthSystem.HealthSystem_C|SetHealth _healthsystem (- (Variables|/Game/Widget/HealthSystem.HealthSystem_C|GetHealth _healthsystem) 1.0)))