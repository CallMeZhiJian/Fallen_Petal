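; SpawnArea is an arena trigger that locks the player in a walled fight and spawns waves of AI enemies.
; Its first overlap, if by the player, spawns a wave and enables wall collision.
; Waves come from a map of enemy types and counts, placed at successive spline points.
; An enemy-count-zero event triggers each next wave, dropping wall collision once the wave counter exceeds the map size.
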(event Custom|SpawnNextWave
  (if (<= (Variables|Default|GetWaveCount) (Utilities|Map|Length (Variables|Default|GetWave)))
    (CallFunction|SpawnEnemy (Variables|Default|GetWaveCount))
    (else
      (CallFunction|DisableFightArea))))

(event EventBeginPlay
  (EventDispatchers|BindEventtoOnEnemyCountZero (delegate Custom|SpawnNextWave)))

(event Collision|EventActorBeginOverlap
  (params (OtherActor :type Actor%20Object%20Reference))
  (Utilities|FlowControl|DoOnce false
    (:Completed
      (if (== OtherActor (Game|GetPlayerCharacter 0))
        (CallFunction|SpawnEnemy (Variables|Default|GetWaveCount))
        (CallFunction|EnableFightArea)))))

(fn ConstructionScript)

(fn SpawnEnemy
  (params (WaveNumber :type Integer))
  (bind _wave (Variables|Default|GetWave))
  (bind (_value _returnvalue) (Utilities|Map|Find _wave WaveNumber))
  (if _returnvalue
    (for _index (range 0 1)
      (for _index_2 (range 1 (Utilities|Array|Get(acopy) (Variables|/Game/Blueprints/AI/SpawnData.SpawnData_C|GetNumberOfEnemy _value) _index))
        (AI|SpawnAIFromClass (Utilities|Array|Get(acopy) (Variables|/Game/Blueprints/AI/SpawnData.SpawnData_C|GetEnemyType _value) _index) 0 (Spline|GetLocationatSplinePoint (Variables|Default|GetSpawnPoint) (Math|Integer|SelectInt 0 (Variables|Default|GetSpawnPointCount) (== (Variables|Default|GetSpawnPointCount) (Spline|GetNumberOfSplinePoints (Variables|Default|GetSpawnPoint)))) "World") "0, 0, 0" false 0)
        (Variables|Default|SetEnemyCount (+ (Variables|Default|GetEnemyCount) 1))
        (Variables|Default|SetSpawnPointCount (+ (Variables|Default|GetSpawnPointCount) 1))))
    (Variables|Default|SetWaveCount (+ (Variables|Default|GetWaveCount) 1))
    (return true)
    (else
      (Development|PrintString "No Next Wave"))))

(fn EnableFightArea
  (Collision|SetCollisionEnabled (Variables|Default|GetWall1) "QueryAndPhysics"))

(fn DisableFightArea
  (Collision|SetCollisionEnabled (Variables|Default|GetWall1) "NoCollision"))