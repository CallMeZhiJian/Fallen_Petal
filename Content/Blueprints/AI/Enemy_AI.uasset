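; Enemy AI controller that starts the behavior tree assigned on each possessed BP_Enemy_Base pawn.
; After a short delay, it runs the tree and sets the first player character as attack target, stored in both the Blackboard and a variable.
; It then queries the pawn for its ideal attack and defend radii and writes them to the Blackboard.
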(event EventPossess
  (params (PossessedPawn :type Pawn%20Object%20Reference))
  (bind _asbp_enemy_base (Utilities|Casting|CastToBP_Enemy_Base PossessedPawn))
  (bind _behaviortree (Variables|/Game/Blueprints/AI/EnemyBlueprint/BP_Enemy_Base.BP_Enemy_Base_C|GetBehaviorTree _asbp_enemy_base)
    (:then
      (Utilities|FlowControl|Delay 0.2)
      (AI|RunBehaviorTree _behaviortree)
      (CallFunction|SetAttackTarget (Game|GetPlayerCharacter 0))
      (bind (_attackradius _defendradius) (Class|EnemyInterface|GetIdealRange(Message) PossessedPawn))
      (AI|Components|Blackboard|SetValueasFloat (Variables|Default|GetBlackboard) (Variables|Default|GetAttack%20Raduis%20Key%20Name) _attackradius)
      (AI|Components|Blackboard|SetValueasFloat (Variables|Default|GetBlackboard) (Variables|Default|GetDefend%20Radius%20Key%20Name) _defendradius))
    (:else
      (Development|PrintString "No Valid"))))

(fn ConstructionScript)

(fn SetAttackTarget
  (params (AttackTarget :type Actor%20Object%20Reference))
  (AI|Components|Blackboard|SetValueasObject (Variables|Default|GetBlackboard) (Variables|Default|GetAttackTargetName) AttackTarget)
  (Variables|Default|SetAttack%20Target AttackTarget))