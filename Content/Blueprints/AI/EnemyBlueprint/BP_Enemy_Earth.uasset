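; BP_Enemy_Earth is an enemy AI Blueprint providing two montage-driven attacks, a charge and an area-of-effect blast, that report through OnAttackEnd.
; On montage notify, the charge boosts walk speed and moves forward while a Timeline sphere-traces, spawning explosions on hits; speed drops on move success.
; The AOE notify spawns a large explosion and runs a wide debug-drawn trace whose result is unused; neither attack applies damage here.
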(event EventChargeAttack
  (bind _returnvalue (Transformation|GetActorLocation))
  (Development|PrintString "ChargeAttack")
  (Animation|Montage|PlayMontage (Variables|Character|GetMesh) "/Game/Blueprints/AI/Animation/ImportedAnimation/Creature/Running_Crawl_Montage.Running_Crawl_Montage"
    (:OnCompleted
      (Default|CallOnAttackEnd :!label _label))
    (:OnInterrupted
      (goto _label))
    (:OnNotifyBegin
      (Variables|/Script/Engine.CharacterMovementComponent|SetMaxWalkSpeed (Variables|Character|GetCharacterMovement) 2e+03)
      (AI|AIMoveTo self (+ (Transformation|GetActorLocation) (* (Transformation|GetActorForwardVector) 7.5e+02)) 0 5.0 false
        (:then
          (Timeline|Timeline PlayFromStart
            (:Update
              (bind (_outhit _returnvalue_2) (Collision|SphereTraceForObjects _returnvalue _returnvalue 1e+02 (Utilities|Array|MakeArray "ObjectTypeQuery7") false 0 "ForOneFrame" true "(R=1.000000,G=0.000000,B=0.000000,A=1.000000)" "(R=0.000000,G=1.000000,B=0.000000,A=1.000000)" 1.0))
              (if _returnvalue_2
                (Effects|SpawnEmitteratLocation "/Game/StarterContent/Particles/P_Explosion.P_Explosion" (.TraceEnd (Collision|BreakHitResult _outhit)))))))
        (:OnSuccess
          (Variables|/Script/Engine.CharacterMovementComponent|SetMaxWalkSpeed (Variables|Character|GetCharacterMovement) 5e+02))))))

(event EventAOEAttack
  (bind _returnvalue (Transformation|GetActorLocation))
  (Animation|Montage|PlayMontage (Variables|Character|GetMesh) "/Game/Blueprints/AI/Animation/ImportedAnimation/Creature/Standing_Taunt_Battlecry_Montage.Standing_Taunt_Battlecry_Montage"
    (:OnCompleted
      (Default|CallOnAttackEnd))
    (:OnNotifyBegin
      (Effects|SpawnEmitteratLocation "/Game/StarterContent/Particles/P_Explosion.P_Explosion" (Transformation|GetActorLocation) "0, 0, 0" "10.000000,10.000000,10.000000")
      (Collision|SphereTraceForObjects _returnvalue _returnvalue 5e+02 (Utilities|Array|MakeArray "ObjectTypeQuery7") false 0 "ForDuration"))))

(fn ConstructionScript
  (|CallParentFunction))