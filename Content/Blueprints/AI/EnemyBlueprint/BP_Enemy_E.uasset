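; BP_Enemy_E is an enemy character with two montage-driven attacks, a forward charge and an area slam, both ending by calling OnAttackEnd.
; On montage notify, the charge boosts walk speed, moves forward via AIMoveTo and enables a collision that damages the player on overlap.
; The slam's notify spawns a large explosion and sphere-traces to damage one target with knockback, leaving debug drawing on.
; KnockbackPlayer launches a target away from the enemy.
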(event OnComponentBeginOverlap(ChargeCollision)
  (params (OverlappedComponent :type Primitive%20Component%20Object%20Reference) (OtherActor :type Actor%20Object%20Reference) (OtherComp :type Primitive%20Component%20Object%20Reference) (OtherBodyIndex :type Integer) (bFromSweep :type Boolean) (SweepResult :type Hit%20Result%20Structure%20%28by%20ref%29))
  (bind _returnvalue (Game|GetPlayerCharacter 0))
  ;[1 1 1] Charge Collision Check
  (if (== OtherActor _returnvalue)
    (Effects|SpawnEmitteratLocation "/Game/StarterContent/Particles/P_Explosion.P_Explosion" (Transformation|GetActorLocation _returnvalue) "0, 0, 0" "2.000000,2.000000,2.000000")
    (CallFunction|DamageTarget (Game|GetPlayerCharacter 0) 1e+01 false 2e+01)))

(event Custom|Knockback%20Player
  (params (Target :type Character%20Object%20Reference))
  (Character|LaunchCharacter Target (* (- (Transformation|GetActorLocation Target) (Transformation|GetActorLocation)) 1e+01) true true))

(event EventChargeAttack
  ;[1 1 1] Charge Attack
  (Animation|Montage|PlayMontage (Variables|Character|GetMesh) "/Game/Blueprints/AI/Animation/ImportedAnimation/Creature/Running_Crawl_Montage.Running_Crawl_Montage"
    (:OnCompleted
      (Default|CallOnAttackEnd :!label _label)
      (Collision|SetCollisionEnabled (Variables|Default|GetChargeCollision) "NoCollision"))
    (:OnInterrupted
      (goto _label))
    (:OnNotifyBegin
      (Variables|/Script/Engine.CharacterMovementComponent|SetMaxWalkSpeed (Variables|Character|GetCharacterMovement) 2e+03)
      (AI|AIMoveTo self (+ (Transformation|GetActorLocation) (* (Transformation|GetActorForwardVector) 7.5e+02)) 0 5.0 false
        (:then
          (Collision|SetCollisionEnabled (Variables|Default|GetChargeCollision) "QueryAndPhysics"))
        (:OnSuccess
          (Variables|/Script/Engine.CharacterMovementComponent|SetMaxWalkSpeed (Variables|Character|GetCharacterMovement) 5e+02))))))

(event EventAOEAttack
  (bind _returnvalue (Transformation|GetActorLocation))
  ;[1 1 1] AOE Attack
  (Animation|Montage|PlayMontage (Variables|Character|GetMesh) "/Game/Blueprints/AI/Animation/ImportedAnimation/Creature/Standing_Taunt_Battlecry_Montage.Standing_Taunt_Battlecry_Montage"
    (:OnCompleted
      (Default|CallOnAttackEnd))
    (:OnNotifyBegin
      (Effects|SpawnEmitteratLocation "/Game/StarterContent/Particles/P_Explosion.P_Explosion" (Transformation|GetActorLocation) "0, 0, 0" "10.000000,10.000000,10.000000")
      (bind (_outhit _returnvalue_2) (Collision|SphereTraceForObjects _returnvalue _returnvalue 5e+02 (Utilities|Array|MakeArray "ObjectTypeQuery7") false 0 "ForDuration"))
      (if _returnvalue_2
        (CallFunction|DamageTarget (.HitActor (Collision|BreakHitResult _outhit)) 1e+01 true 1e+01)))))

(fn ConstructionScript
  (|CallParentFunction))