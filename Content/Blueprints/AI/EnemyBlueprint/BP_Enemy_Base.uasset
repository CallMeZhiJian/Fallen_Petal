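; Base enemy character for AI combat, providing attack, damage, hit-reaction, sword-wielding, ideal-range and movement-speed functions.
; Taking damage writes its state to the Blackboard and refreshes a health bar widget from HealthSystem.
; Attacks reserve tokens from the level's CombatSystem actor and return them on AttackEnd, while its own CombatTokenSystem handles token requests made on this enemy.
; DamageTarget applies damage and can launch the main character away as knockback.
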(event Custom|TakeDamage
  (params (DamagedActor :type Actor%20Object%20Reference) (Damage :type Float%20%28single-precision%29) (DamageType :type Damage%20Type%20Object%20Reference) (InstigatedBy :type Controller%20Object%20Reference) (DamageCauser :type Actor%20Object%20Reference))
  (AI|Components|Blackboard|SetValueasEnum (AI|GetBlackboard 0) (Variables|Default|GetStatesName) (Variables|Default|GetStates))
  (CallFunction|UpdateHealthBar))

(event Custom|WieldSword
  (bind _returnvalue (Game|SpawnActorfromClass "/Game/Blueprints/AI/Animation/Weapon/Sword.Sword_C" (Transformation|GetActorTransform) "Undefined" "MultiplyWithRoot" 0 0))
  (Transformation|AttachComponentToComponent _returnvalue (Variables|Character|GetMesh) "hand_r_sword_socket" "SnapToTarget" "SnapToTarget" "SnapToTarget" true))

(event EventBeginPlay
  (EventDispatchers|BindEventtoOnTakeAnyDamage (delegate Custom|TakeDamage))
  (CallFunction|UpdateHealthBar))

(event EventHitReaction
  (Animation|Montage|PlayMontage (Variables|Character|GetMesh) (Variables|Default|GetHitMontage)
    (:OnCompleted
      _)
    (:OnInterrupted
      _))
  (Default|CallOnHitReactEnd))

(event EventReturnToken
  (params (Amount :type Integer))
  (Default|ReturnToken (Variables|Default|GetCombatTokenSystem) Amount))

(event EventAttackEnd
  (params (AttackTarget :type Actor%20Object%20Reference))
  (bind _returnvalue (Actor|GetActorOfClass "/Game/Blueprints/AI/EnemyBlueprint/CombatSystem.CombatSystem_C"))
  (Class|EnemyInterface|ReturnToken(Message) _returnvalue (Variables|Default|GetTokenUsedCount)))

(fn ConstructionScript)

(fn UpdateHealthBar
  (bind _aswb_enemy_health_bar (Utilities|Casting|CastToWB_EnemyHealthBar (UserInterface|GetUserWidgetObject (Variables|Default|GetEnemy%20Health%20Bar))))
  (Variables|/Game/Widget/WB_EnemyHealthBar.WB_EnemyHealthBar_C|SetHealth _aswb_enemy_health_bar (Variables|/Game/Widget/HealthSystem.HealthSystem_C|GetHealth (Variables|Default|GetHealthSystem)))
  (return))

(fn AttackStart
  (params (Attack%20Target :type Actor%20Object%20Reference) (TokenNeeded :type Integer))
  (bind _returnvalue (Actor|GetActorOfClass "/Game/Blueprints/AI/EnemyBlueprint/CombatSystem.CombatSystem_C"))
  (bind _success (Class|EnemyInterface|ReserveToken(Message) _returnvalue TokenNeeded))
  (if _success
    (Variables|Default|SetTokenUsedCount TokenNeeded)
    (return true)
    (else
      (Development|PrintString "fail to resreve")
      (return false))))

(fn DamageTarget
  (params (TargetActor :type Actor%20Object%20Reference) (Damage :type Float%20%28double-precision%29) (Knockback? :type Boolean) (KnockbackStrength :type Float%20%28double-precision%29))
  (Game|Damage|ApplyDamage TargetActor Damage 0 0)
  (if Knockback?
    (bind _asbp_main_character (Utilities|Casting|CastToBP_MainCharacter TargetActor))
    (Character|LaunchCharacter _asbp_main_character (* (- (Transformation|GetActorLocation TargetActor) (Transformation|GetActorLocation)) KnockbackStrength) true true)
    (return true)
    (else
      (return true))))

(fn GetIdealRange
  (return 1.5e+02 5e+02))

(fn ReserveToken
  (params (Amount :type Integer))
  (bind _success (Default|ReserveToken (Variables|Default|GetCombatTokenSystem) Amount))
  (return _success))

(fn SetMovementSpeed
  (params (Speed :type E_MovementSpeed%20Enum :default "NewEnumerator0"))
  (bind _output_get (Variables|/Script/Engine.CharacterMovementComponent|SetMaxWalkSpeed (Variables|Character|GetCharacterMovement) (Utilities|Select :Index Speed :NewEnumerator0 0.0 :NewEnumerator1 1e+02 :NewEnumerator2 3e+02 :NewEnumerator3 5e+02)))
  (return _output_get))