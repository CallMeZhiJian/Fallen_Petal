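; Creature enemy Blueprint holding two draft attacks, both unreachable as nothing triggers them.
; The charge plays a crawl montage whose notify boosts speed, moves the creature forward by AI and runs timeline-driven sphere traces that spawn explosions on pawn hits.
; The battlecry montage's notify spawns a large explosion and a wide pawn trace with its result unused.
; Both signal attack end on montage completion, the charge also on interruption; neither applies damage.
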(fn ConstructionScript
  (|CallParentFunction))