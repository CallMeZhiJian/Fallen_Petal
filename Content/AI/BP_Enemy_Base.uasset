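; Base enemy character that spawns a sword into its hand socket and performs token-gated melee attacks.
; AttackStart reserves tokens from the target; AttackEnd returns them once the slash montage completes or is interrupted.
; A montage notify runs a forward sphere trace for pawns, which only spawns an explosion and prints on hit.
; It also exposes its own CombatTokenSystem, ideal combat ranges and speed presets.
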(event Custom|WieldSword
  (bind _returnvalue (Game|SpawnActorfromClass "/Game/AI/Animation/Weapon/Sword.Sword_C" (Transformation|GetActorTransform) "Undefined" "MultiplyWithRoot" 0 0))
  (Transformation|AttachComponentToComponent _returnvalue (Variables|Character|GetMesh) "hand_r_sword_socket" "SnapToTarget" "SnapToTarget" "SnapToTarget" true))

(event EventBeginPlay
  (CallFunction|WieldSword))

(event EventReturnToken
  (params (Amount :type Integer))
  (Default|ReturnToken (Variables|Default|GetCombatTokenSystem) Amount))

(event EventAttack
  (params (AttackTarget :type Actor%20Object%20Reference))
  (bind _returnvalue (Transformation|GetActorLocation))
  ;[1 1 1] Attack
  (Animation|Montage|PlayMontage (Variables|Character|GetMesh) "/Game/AI/Animation/EnemyAnimation/Manny_Sword_And_Shield_Slash_Anim_mixamo_com_Montage.Manny_Sword_And_Shield_Slash_Anim_mixamo_com_Montage"
    (:OnCompleted
      (CallFunction|AttackEnd AttackTarget :!label _label))
    (:OnInterrupted
      (goto _label))
    (:OnNotifyBegin
      (bind (_outhit _returnvalue_2) (Collision|SphereTraceForObjects _returnvalue (+ _returnvalue (* (Transformation|GetActorForwardVector) 1.5e+02)) 2e+01 (Utilities|Array|MakeArray "ObjectTypeQuery3") false 0 "ForDuration" true "(R=1.000000,G=0.000000,B=0.000000,A=1.000000)" "(R=0.000000,G=1.000000,B=0.000000,A=1.000000)" 1.0))
      (if _returnvalue_2
        (Effects|SpawnEmitteratLocation "/Game/StarterContent/Particles/P_Explosion.P_Explosion" (.TraceEnd (Collision|BreakHitResult _outhit)))
        (Development|PrintString "Hit")))))

(event EventAttackEnd
  (params (AttackTarget :type Actor%20Object%20Reference))
  (Class|EnemyInterface|ReturnToken(Message) AttackTarget (Variables|Default|GetTokenUsedCount))
  (Default|CallOnAttackEnd))

(fn ConstructionScript)

(fn AttackStart
  (params (Attack%20Target :type Actor%20Object%20Reference) (TokenNeeded :type Integer))
  (bind _success (Class|EnemyInterface|ReserveToken(Message) Attack%20Target TokenNeeded))
  (if _success
    (Variables|Default|SetTokenUsedCount TokenNeeded)
    (return true)
    (else
      (return false))))

(fn GetIdealRange
  (return 1.5e+02 3.5e+02))

(fn ReserveToken
  (params (Amount :type Integer))
  (bind _success (Default|ReserveToken (Variables|Default|GetCombatTokenSystem) Amount))
  (return _success))

(fn SetMovementSpeed
  (params (Speed :type E_MovementSpeed%20Enum :default "NewEnumerator0"))
  (bind _output_get (Variables|/Script/Engine.CharacterMovementComponent|SetMaxWalkSpeed (Variables|Character|GetCharacterMovement) (Utilities|Select :Index Speed :NewEnumerator0 0.0 :NewEnumerator1 1e+02 :NewEnumerator2 3e+02 :NewEnumerator3 5e+02)))
  (return _output_get))