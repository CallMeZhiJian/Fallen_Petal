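; Base AI projectile that launches toward a target actor and reports what it hits.
; Construction applies Speed to the projectile movement component's initial and max speed.
; On BeginPlay it ignores its owner while moving and, if a target is valid, aims velocity at it once, without homing.
; A box collision hit fires the OnProjectileHIt dispatcher, spawns effect and sound, then destroys the projectile.
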(event OnComponentHit(BoxCollision)
  (params (HitComponent :type Primitive%20Component%20Object%20Reference) (OtherActor :type Actor%20Object%20Reference) (OtherComp :type Primitive%20Component%20Object%20Reference) (NormalImpulse :type Vector :default "0, 0, 0") (Hit :type Hit%20Result%20Structure%20%28by%20ref%29))
  (bind _location (Collision|BreakHitResult Hit))
  (Default|CallOnProjectileHIt OtherActor Hit)
  (Effects|SpawnEmitteratLocation (Variables|Effect|GetHitEffect) _location)
  (Audio|PlaySoundatLocation (Variables|Sound|GetHitSound) _location "0, 0, 0" 1.0 1.0 0.0 0 0 0 0)
  (Actor|DestroyActor))

(event Custom|RotateToActor
  (Variables|/Script/Engine.MovementComponent|SetVelocity (Variables|Default|GetProjectileMovement) (* (Math|Vector|GetUnitDirection(Vector) (Transformation|GetActorLocation) (Transformation|GetActorLocation (Variables|Target|GetTargetActor))) (Variables|ProjectileSetting|GetSpeed))))

(event EventBeginPlay
  (Collision|IgnoreActorwhenMoving (Variables|Default|GetBoxCollision) (Components|GetOwner) true)
  (Variables|Target|GetTargetActor
    (:then
      (CallFunction|RotatetoActor))
    (:else)))

(fn ConstructionScript
  (bind _projectilemovement (Variables|Default|GetProjectileMovement))
  (Variables|/Script/Engine.ProjectileMovementComponent|SetInitialSpeed _projectilemovement (Variables|ProjectileSetting|GetSpeed))
  (Variables|/Script/Engine.ProjectileMovementComponent|SetMaxSpeed _projectilemovement (Variables|ProjectileSetting|GetSpeed)))