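; Melee enemy Blueprint that wields a sword on BeginPlay and provides sword and magic attack events.
; Attack plays a slash montage whose notify sphere-traces forward for pawns, ignoring other enemies; hits only spawn an explosion and print debug text.
; MagicAttack plays a casting montage whose notify spawns a projectile from the right hand at the target.
; Both montages end the attack and fire their end callbacks, whether completed or interrupted.
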(event EventBeginPlay
  (CallFunction|WieldSword))

(event EventMagicAttack
  (params (AttackTarget :type Actor%20Object%20Reference))
  ;[1 1 1] Magic Attack
  (Animation|Montage|PlayMontage (Variables|Character|GetMesh) "/Game/AI/Animation/EnemyAnimation/Manny_Magic_Heal_Montage.Manny_Magic_Heal_Montage"
    (:OnCompleted
      (CallFunction|AttackEnd AttackTarget :!label _label)
      (Default|CallOnSpellEnd))
    (:OnInterrupted
      (goto _label))
    (:OnNotifyBegin
      (bind _returnvalue (Game|SpawnActorfromClass "/Game/AI/Projectile/BP_Projectile_Base_MagicSpell.BP_Projectile_Base_MagicSpell_C" (Transformation|GetSocketTransform (Variables|Character|GetMesh) "hand_r" "RTS_World") "Undefined" "MultiplyWithRoot" self 5e+02 0 "/Game/StarterContent/Audio/Explosion_Cue.Explosion_Cue" AttackTarget 0))
      (Collision|IgnoreActorwhenMoving (Variables|Default|GetCapsuleComponent) _returnvalue true))))

(event EventAttack
  (params (AttackTarget :type Actor%20Object%20Reference))
  (bind _returnvalue (Transformation|GetActorLocation))
  ;[1 1 1] Attack
  (Animation|Montage|PlayMontage (Variables|Character|GetMesh) "/Game/AI/Animation/EnemyAnimation/Manny_Sword_And_Shield_Slash_Anim_mixamo_com_Montage.Manny_Sword_And_Shield_Slash_Anim_mixamo_com_Montage"
    (:OnCompleted
      (CallFunction|AttackEnd AttackTarget :!label _label)
      (Default|CallOnAttackEnd))
    (:OnInterrupted
      (goto _label))
    (:OnNotifyBegin
      (bind _outactors (Actor|GetAllActorsOfClass "/Game/AI/EnemyBlueprint/BP_Enemy_Base.BP_Enemy_Base_C"))
      (bind (_outhit _returnvalue_2) (Collision|SphereTraceForObjects _returnvalue (+ _returnvalue (* (Transformation|GetActorForwardVector) 1.5e+02)) 2e+01 (Utilities|Array|MakeArray "ObjectTypeQuery3") false _outactors "ForDuration" true "(R=1.000000,G=0.000000,B=0.000000,A=1.000000)" "(R=0.000000,G=1.000000,B=0.000000,A=1.000000)" 1.0))
      (if _returnvalue_2
        (Effects|SpawnEmitteratLocation "/Game/StarterContent/Particles/P_Explosion.P_Explosion" (.TraceEnd (Collision|BreakHitResult _outhit)))
        (Development|PrintString "Hit")))))

(fn ConstructionScript
  (|CallParentFunction))