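; BP_Enemy_Base is the base enemy character, providing shared combat and movement functions for enemy AI.
; AttackStart reserves tokens from CombatTokenSystem and records the amount, and AttackEnd returns them, gating attacks on token availability.
; WieldSword spawns a sword and snaps it to the right-hand socket.
; Helpers report fixed attack and defend ranges and map speed states to max walk speed.
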(event Custom|WieldSword
  (bind _returnvalue (Game|SpawnActorfromClass "/Game/AI/Animation/Weapon/Sword.Sword_C" (Transformation|GetActorTransform) "Undefined" "MultiplyWithRoot" 0 0))
  (Transformation|AttachComponentToComponent _returnvalue (Variables|Character|GetMesh) "hand_r_sword_socket" "SnapToTarget" "SnapToTarget" "SnapToTarget" true))

(event EventReturnToken
  (params (Amount :type Integer))
  (Default|ReturnToken (Variables|Default|GetCombatTokenSystem) Amount))

(event EventAttackEnd
  (params (AttackTarget :type Actor%20Object%20Reference))
  (CallFunction|ReturnToken (Variables|Default|GetTokenUsedCount)))

(fn ConstructionScript)

(fn AttackStart
  (params (Attack%20Target :type Actor%20Object%20Reference) (TokenNeeded :type Integer))
  (bind _success (CallFunction|ReserveToken TokenNeeded))
  (if _success
    (Variables|Default|SetTokenUsedCount TokenNeeded)
    (return true)
    (else
      (return false))))

(fn GetIdealRange
  (return 1.5e+02 5e+02))

(fn ReserveToken
  (params (Amount :type Integer))
  (bind _success (Default|ReserveToken (Variables|Default|GetCombatTokenSystem) Amount))
  (return _success))

(fn SetMovementSpeed
  (params (Speed :type E_MovementSpeed%20Enum :default "NewEnumerator0"))
  (bind _output_get (Variables|/Script/Engine.CharacterMovementComponent|SetMaxWalkSpeed (Variables|Character|GetCharacterMovement) (Utilities|Select :Index Speed :NewEnumerator0 0.0 :NewEnumerator1 1e+02 :NewEnumerator2 3e+02 :NewEnumerator3 5e+02)))
  (return _output_get))